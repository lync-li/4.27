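; Editor tool Blueprint that bakes a two-color gradient ramp texture from configurable dark and light colors.
; Bake creates a dynamic instance of the Ramp_Gradual material, sets both colors, and draws it into a new square float render target of configurable size.
; It exports that target to the configured path and file name as .hdr, then redraws the material into the Preview render target if one is valid.
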(fn `Bake`
  (bind `_尺寸` (`self.尺寸`))
  (bind _preview (`self.Preview`))
  (`|ExecutionSequence`
    (:`then_0`
      (bind _returnvalue (`KismetMaterialLibrary.CreateDynamicMaterialInstance` "/Game/Tool/生成渐变图_设置颜色版/Ramp_Gradual.Ramp_Gradual"))
      (bind _output_get (set `self.CMDI` _returnvalue))
      (`MaterialInstanceDynamic.SetVectorParameterValue` _output_get "DarkerColor" (`self.DarkerColor`))
      (`MaterialInstanceDynamic.SetVectorParameterValue` _output_get "LightColor" (`self.LightColor`)))
    (:`then_1`
      (bind _returnvalue_2 (`KismetRenderingLibrary.CreateRenderTarget2D` `_尺寸` `_尺寸`))
      (bind _output_get_2 (set `self.RenderTaget` _returnvalue_2))
      (`KismetRenderingLibrary.DrawMaterialToRenderTarget` _output_get_2 (`self.CMDI`)))
    (:`then_2`
      (`KismetRenderingLibrary.ExportRenderTarget` (`self.RenderTaget`) (`self.保存路径`) (`KismetStringLibrary.Concat_StrStr` (`self.保存文件名`) ".hdr")))
    (:`then_3`
      (`/Engine/EditorBlueprintResources/StandardMacros.IsValid` _preview
        (:`Is Valid`
          (`KismetRenderingLibrary.DrawMaterialToRenderTarget` _preview (`self.CMDI`)))))))

(fn `UserConstructionScript`)