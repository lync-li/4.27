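; BP_CraetRamp_v3 is an editor tool that bakes gradient ramp textures, the curve-based version per its folder name.
; Bake feeds the input texture into a dynamic Ramp_Gradual material as RampColor and draws it to a new square render target.
; It exports that target as an HDR file using the configured path and name.
; If Preview is valid, it also draws there and saves the baked target as a static texture named by hour and minute.
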(fn `Bake`
  (bind `_尺寸` (`self.尺寸`))
  (bind _preview (`self.Preview`))
  (bind (_year _month _day _hour _minute) (`KismetMathLibrary.BreakDateTime` (`KismetMathLibrary.GetDate` (struct))))
  (`|ExecutionSequence`
    (:`then_0`
      (bind _returnvalue (`KismetMaterialLibrary.CreateDynamicMaterialInstance` "/Game/Tool/生成渐变图_曲线版/Ramp_Gradual.Ramp_Gradual"))
      (bind _output_get (set `self.CMDI` _returnvalue))
      (`MaterialInstanceDynamic.SetTextureParameterValue` _output_get "RampColor" (`self.Texture`)))
    (:`then_1`
      (bind _returnvalue_2 (`KismetRenderingLibrary.CreateRenderTarget2D` `_尺寸` `_尺寸`))
      (bind _output_get_2 (set `self.RenderTaget` _returnvalue_2))
      (`KismetRenderingLibrary.DrawMaterialToRenderTarget` _output_get_2 (`self.CMDI`)))
    (:`then_2`
      (`KismetRenderingLibrary.ExportRenderTarget` (`self.RenderTaget`) (`self.保存路径`) (`KismetStringLibrary.Concat_StrStr` (`self.保存文件名`) ".hdr")))
    (:`then_3`
      (`/Engine/EditorBlueprintResources/StandardMacros.IsValid` _preview
        (:`Is Valid`
          (`KismetRenderingLibrary.DrawMaterialToRenderTarget` _preview (`self.CMDI`))
          (`KismetRenderingLibrary.RenderTargetCreateStaticTexture2DEditorOnly` _output_get_2 (`KismetStringLibrary.Concat_StrStr` (`KismetStringLibrary.Conv_IntToString` _hour) (`KismetStringLibrary.Conv_IntToString` _minute))))))))

(fn `UserConstructionScript`)