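; A demo player camera manager that feeds the camera's world transform to self-lighting static mesh actors.
; Every tick it finds all SelfLightingStaticMesh actors and calls NotifyCameraTransform on each with its transform component's world transform.
; The construction script does the same for a single such actor.
; A similar loop for SelfLightingSkeletonMesh actors is present but unconnected, so it never runs.
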(event `self.ReceiveTick`
  (params (DeltaSeconds :type "Float (single-precision)"))
  (bind _outactors (`GameplayStatics.GetAllActorsOfClass` "/Game/StarterContent/Actor/BluePrints/SelfLightingStaticMesh.SelfLightingStaticMesh_C"))
  (for _array_element _outactors
    (bind _asself_lighting_static_mesh (cast `/Game/StarterContent/Actor/BluePrints/SelfLightingStaticMesh` _array_element))
    (`/Game/StarterContent/Actor/BluePrints/SelfLightingStaticMesh.NotifyCameraTransform` _asself_lighting_static_mesh (`SceneComponent.K2_GetComponentToWorld` (`self.TransformComponent`)))))

(fn `UserConstructionScript`
  (bind _returnvalue (`GameplayStatics.GetActorOfClass` "/Game/StarterContent/Actor/BluePrints/SelfLightingStaticMesh.SelfLightingStaticMesh_C"))
  (`/Game/StarterContent/Actor/BluePrints/SelfLightingStaticMesh.NotifyCameraTransform` _returnvalue (`SceneComponent.K2_GetComponentToWorld` (`self.TransformComponent`))))