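; Directional light Blueprint that publishes its sun direction and color to materials through the LightDirCollection material parameter collection.
; Every Tick, and in the construction script for editor updates, it writes LightDir as the negated forward vector of its directional light component.
; It also writes LightColor as the light color scaled by intensity and divided by Pi.
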(event `self.ReceiveTick`
  (params (DeltaSeconds :type "Float (single-precision)"))
  (bind _directional_light (`self.Directional LIght`))
  (`KismetMaterialLibrary.SetVectorParameterValue` "/Game/_Global/Materials/Collection/LightDirCollection.LightDirCollection" "LightDir" (`KismetMathLibrary.Conv_VectorToLinearColor` (* (`SceneComponent.GetForwardVector` (`self.Directional LIght`)) -1.0)))
  (`KismetMaterialLibrary.SetVectorParameterValue` "/Game/_Global/Materials/Collection/LightDirCollection.LightDirCollection" "LightColor" (`KismetMathLibrary.Conv_VectorToLinearColor` (/ (`KismetMathLibrary.Conv_LinearColorToVector` (* (`LightComponentBase.GetLightColor` _directional_light) (`LightComponentBase.Intensity` _directional_light))) (`KismetMathLibrary.GetPI`)))))

(fn `UserConstructionScript`
  (bind _directional_light (`self.Directional LIght`))
  (`KismetMaterialLibrary.SetVectorParameterValue` "/Game/_Global/Materials/Collection/LightDirCollection.LightDirCollection" "LightDir" (`KismetMathLibrary.Conv_VectorToLinearColor` (* (`SceneComponent.GetForwardVector` _directional_light) -1.0)))
  (`KismetMaterialLibrary.SetVectorParameterValue` "/Game/_Global/Materials/Collection/LightDirCollection.LightDirCollection" "LightColor" (`KismetMathLibrary.Conv_VectorToLinearColor` (/ (`KismetMathLibrary.Conv_LinearColorToVector` (* (`LightComponentBase.GetLightColor` _directional_light) (`LightComponentBase.Intensity` _directional_light))) (`KismetMathLibrary.GetPI`)))))